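; BP_DoorForward is a door that swings open automatically when the third-person character enters its trigger.
; On overlap, it compares a normalized location difference with the door's forward vector, using a loose tolerance, to choose the swing direction.
; The DoorTimer timeline then drives the SMDoor mesh's relative yaw by a signed Angle.
; Leaving the trigger only clears CanInteract, with no closing logic.
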(event `self.Trigger.OnComponentBeginOverlap`
  (params (OverlappedComponent :type "PrimitiveComponent Object Reference") (OtherActor :type "Actor Object Reference") (OtherComp :type "PrimitiveComponent Object Reference") (OtherBodyIndex :type Integer) (bFromSweep :type Boolean) (SweepResult :type "HitResult Structure (by ref)"))
  (cast `/Game/ThirdPerson/Blueprints/BP_ThirdPersonCharacter` OtherActor)
  (set `self.CanInteract` true)
  (if true
    (set `self.Direction` (== (`KismetMathLibrary.Normal` (- (`self.K2_GetActorLocation`) (`self.K2_GetActorLocation`))) (`self.GetActorForwardVector`) :`ErrorTolerance` 1.0))
    (bind (_direction _doortimer) (`Timeline|DoorTimer`)
      (:`Update`
        (`SceneComponent.K2_SetRelativeRotation` (`self.SM_Door`) (`KismetMathLibrary.MakeRotator` 0.0 0.0 (* _doortimer (`self.Angle`) (`KismetMathLibrary.SelectFloat` 1.0 -1.0 (`self.Direction`)))) false false)))))

(event `self.Trigger.OnComponentEndOverlap`
  (params (OverlappedComponent :type "PrimitiveComponent Object Reference") (OtherActor :type "Actor Object Reference") (OtherComp :type "PrimitiveComponent Object Reference") (OtherBodyIndex :type Integer))
  (cast `/Game/ThirdPerson/Blueprints/BP_ThirdPersonCharacter` OtherActor)
  (set `self.CanInteract` false))

(fn `UserConstructionScript`)